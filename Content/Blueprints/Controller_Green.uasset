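; Player controller that rolls the ball of the possessed BP_Pawn_lv1 and steers its view with the mouse.
; BeginPlay caches the pawn, then Tick polls WASD directly and applies mass-independent acceleration to the Ball along the camera's forward and right vectors.
; Mouse X and Y axis events feed yaw and inverted pitch input to the controller's rotation.
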(event EventBeginPlay
  (bind _asbp_pawn_lv_1 (Utilities|Casting|CastToBP_Pawn_lv1 (Pawn|GetControlledPawn)))
  (Variables|Default|SetAs%20BP%20Pawn%20Lv%201 _asbp_pawn_lv_1))

(event EventTick
  (params (DeltaSeconds :type Float%20%28single-precision%29))
  (bind _as_bp_pawn_lv_1 (Variables|Default|GetAs%20BP%20Pawn%20Lv%201))
  (bind _as_bp_pawn_lv_1_2 (Variables|Default|GetAs%20BP%20Pawn%20Lv%201))
  (bind _as_bp_pawn_lv_1_3 (Variables|Default|GetAs%20BP%20Pawn%20Lv%201))
  (bind _as_bp_pawn_lv_1_4 (Variables|Default|GetAs%20BP%20Pawn%20Lv%201))
  (Utilities|FlowControl|Sequence
    (:then_0
      ;[1 1 1] W
      (if (Game|Player|IsInputKeyDown "W")
        (Physics|AddForce (Variables|/Game/Blueprints/BP_Pawn_lv1.BP_Pawn_lv1_C|GetBall _as_bp_pawn_lv_1_2) (* (Math|Vector|GetForwardVector (Variables|/Game/Blueprints/BP_Pawn_lv1.BP_Pawn_lv1_C|GetCamera _as_bp_pawn_lv_1_2)) 1e+03) "None" true)))
    (:then_1
      ;[1 1 1] S
      (if (Game|Player|IsInputKeyDown "S")
        (Physics|AddForce (Variables|/Game/Blueprints/BP_Pawn_lv1.BP_Pawn_lv1_C|GetBall _as_bp_pawn_lv_1_3) (* (Math|Vector|GetForwardVector (Variables|/Game/Blueprints/BP_Pawn_lv1.BP_Pawn_lv1_C|GetCamera _as_bp_pawn_lv_1_3)) -1e+03) "None" true)))
    (:then_2
      ;[1 1 1] A
      (if (Game|Player|IsInputKeyDown "A")
        (Physics|AddForce (Variables|/Game/Blueprints/BP_Pawn_lv1.BP_Pawn_lv1_C|GetBall _as_bp_pawn_lv_1_4) (* (Math|Vector|GetRightVector (Variables|/Game/Blueprints/BP_Pawn_lv1.BP_Pawn_lv1_C|GetCamera _as_bp_pawn_lv_1_4)) -1e+03) "None" true)))
    (:then_3
      ;[1 1 1] D
      (if (Game|Player|IsInputKeyDown "D")
        (Physics|AddForce (Variables|/Game/Blueprints/BP_Pawn_lv1.BP_Pawn_lv1_C|GetBall _as_bp_pawn_lv_1) (* (Math|Vector|GetRightVector (Variables|/Game/Blueprints/BP_Pawn_lv1.BP_Pawn_lv1_C|GetCamera _as_bp_pawn_lv_1)) 1e+03) "None" true)))))

(event Input|MouseEvents|MouseX
  (params (AxisValue :type Float%20%28single-precision%29))
  ;[1 1 1] Mouse X-Y
  (Class|PlayerController|AddYawInput AxisValue))

(event Input|MouseEvents|MouseY
  (params (AxisValue :type Float%20%28single-precision%29))
  ;[1 1 1] Mouse X-Y
  (Class|PlayerController|AddPitchInput (* AxisValue -1.0)))

(fn ConstructionScript)